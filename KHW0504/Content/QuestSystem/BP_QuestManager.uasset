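; BP_QuestManager is an interactable quest giver that runs a three-objective quest: collect every BP_ObjectToFind, open a door and reach the roof.
; Interaction starts the quest, creates the QuestScreen widget and counts the objects in the level.
; AddObjectFound, RoofReached and DoorOpened update the widget and share one completion check.
; QuestState drives the flow, with TextRender prompting a return to complete the quest on a second interaction.
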(event `Start Interaction`
  (switch `/Game/QuestSystem/EQuestState` (`self.QuestState`)
    (:`NewEnumerator0`
      (`|ExecutionSequence`
        (:`then_0`
          (set `self.QuestState` "NewEnumerator1")
          (bind _returnvalue (`|CreateWidget` "/Game/QuestSystem/QuestScreen.QuestScreen_C"))
          (bind _output_get (set `self.QuestWidget` _returnvalue))
          (`UserWidget.AddToViewport` _output_get 0))
        (:`then_1`
          (bind _outactors (`GameplayStatics.GetAllActorsOfClass` "/Game/QuestSystem/BP_ObjectToFind.BP_ObjectToFind_C"))
          (set `self.TotalObjectsFound` (`KismetArrayLibrary.Array_Length` _outactors)))
        (:`then_2`
          (`self.Update Quest Text`)
          (`TextRenderComponent.K2_SetText` (`self.TextRender`) ""))))
    (:`NewEnumerator2`
      (set `self.QuestState` "NewEnumerator3")
      (`Widget.RemoveFromParent` (`self.QuestWidget`))
      (`TextRenderComponent.K2_SetText` (`self.TextRender`) "Quest Complete"))))

(event `Update Quest Text`
  (bind _questwidget (`self.QuestWidget`))
  (set `/Game/QuestSystem/QuestScreen.BlueSignsFound` (`self.ObjectCollected`) _questwidget)
  (set `/Game/QuestSystem/QuestScreen.TotalNumberOfBlueSigns` (`self.TotalObjectsFound`) _questwidget)
  (set `/Game/QuestSystem/QuestScreen.DoorOpened` (`self.OpenDoorObjective`) _questwidget)
  (set `/Game/QuestSystem/QuestScreen.RoofReached` (`self.RoofObjective`) _questwidget))

(event `Add Object Found`
  (`/Engine/EditorBlueprintResources/StandardMacros.IncrementInt` (`self.ObjectCollected`)
    (:`  `
      (`self.Update Quest Text` :!label _label)
      (if (and (== (`self.ObjectCollected`) (`self.TotalObjectsFound`)) (`self.RoofObjective`) (`self.OpenDoorObjective`))
        (set `self.QuestState` "NewEnumerator2")
        (`TextRenderComponent.K2_SetText` (`self.TextRender`) "Comeback Here to <br> complete the quest")))))

(event `Roof Reached`
  (set `self.RoofObjective` true)
  (goto _label))

(event `Door Opened`
  (set `self.OpenDoorObjective` true)
  (goto _label))

(fn `interact`
  (returns (Succese :type Boolean))
  (`self.Start Interaction`)
  (return false))

(fn `UserConstructionScript`)