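; BP_QuestDoor is an interactable quest door that opens only while the quest state is In Progress.
; A trigger volume shows floating text to the ThirdPersonCharacter, prompting either to start a quest first or to press E.
; Interact calls OpenDoor, which notifies the QuestManager and plays a timeline that moves the mesh vertically from its cached starting location.
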(event `self.ReceiveBeginPlay`
  (set `self.StartingLocation` (`SceneComponent.K2_GetComponentLocation` (`self.StaticMeshComponent`))))

(event `OpenDoor`
  (switch `/Game/QuestSystem/EQuestState` (`/Game/QuestSystem/BP_QuestManager.QuestState` (`self.QuestManager`))
    (:`NewEnumerator1`
      (`/Game/QuestSystem/BP_QuestManager.Door Opened` (`self.QuestManager`))
      (bind (_direction _shouuuuu) (`Timeline|DoorOpening`)
        (:`Update`
          (`SceneComponent.K2_SetWorldLocation` (`self.StaticMeshComponent`) (+ (`self.StartingLocation`) (`KismetMathLibrary.MakeVector` 0.0 0.0 _shouuuuu)) false false))))))

(event `self.Trigger.OnComponentBeginOverlap`
  (params (OverlappedComponent :type "PrimitiveComponent Object Reference") (OtherActor :type "Actor Object Reference") (OtherComp :type "PrimitiveComponent Object Reference") (OtherBodyIndex :type Integer) (bFromSweep :type Boolean) (SweepResult :type "HitResult Structure (by ref)"))
  (bind _textrender (`self.TextRender`))
  (cast `/Game/ThirdPersonBP/Blueprints/ThirdPersonCharacter` OtherActor)
  (`SceneComponent.SetVisibility` (`self.TextRender`) true false)
  (switch `/Game/QuestSystem/EQuestState` (`/Game/QuestSystem/BP_QuestManager.QuestState` (`self.QuestManager`)) :!label _label
    (:`NewEnumerator0`
      (`TextRenderComponent.K2_SetText` _textrender "You need to start<br> a quest first"))
    (:`NewEnumerator1`
      (`TextRenderComponent.K2_SetText` _textrender "Press E<br>to Interact"))))

(event `self.Trigger.OnComponentEndOverlap`
  (params (OverlappedComponent :type "PrimitiveComponent Object Reference") (OtherActor :type "Actor Object Reference") (OtherComp :type "PrimitiveComponent Object Reference") (OtherBodyIndex :type Integer))
  (cast `/Game/ThirdPersonBP/Blueprints/ThirdPersonCharacter` OtherActor)
  (`SceneComponent.SetVisibility` (`self.TextRender`) false false)
  (goto _label))

(fn `interact`
  (returns (Succese :type Boolean))
  (`self.OpenDoor`)
  (return true))

(fn `UserConstructionScript`)